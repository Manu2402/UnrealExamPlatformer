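; Bullet pooling component that pre-spawns BP_Bullet actors at BeginPlay and keeps them hidden for reuse.
; GetBullet removes and returns the first pooled bullet, or nothing if it is invalid or the pool is empty, and AddBullet puts bullets back.
; DisableBullet turns off collision, hides the bullet and moves it to the spawn transform.
; EnableBullet restores collision and visibility, then passes a transform through OnBulletEnabledMessage.
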(event `self.ReceiveBeginPlay`
  ;[0 0 0] Object pooling pattern
  (for _ (range (`self.MaxBullets`))
    (bind _returnvalue (`|SpawnActorFromClass` "/Game/Blueprints/Bullets/BP_Bullet.BP_Bullet_C" (`self.Spawn Transform`) "AlwaysSpawn" "MultiplyWithRoot" null null))
    (`self.DisableBullet` _returnvalue)
    (`KismetArrayLibrary.Array_Add` (`self.Bullets`) _returnvalue)))

(fn `AddBullet`
  (params (Bullet :type "/Game/Blueprints/Bullets/BP_Bullet Object Reference"))
  (`/Engine/EditorBlueprintResources/StandardMacros.IsValid` Bullet
    (:`Is Valid`
      (if (<= (`KismetArrayLibrary.Array_Length` (`self.Bullets`)) (`self.MaxBullets`))
        (`KismetArrayLibrary.Array_Add` (`self.Bullets`) Bullet)))))

(fn `DisableBullet`
  (params (Bullet :type "/Game/Blueprints/Bullets/BP_Bullet Object Reference"))
  (`/Engine/EditorBlueprintResources/StandardMacros.IsValid` Bullet
    (:`Is Valid`
      (`Actor.SetActorEnableCollision` Bullet false)
      (`Actor.SetActorHiddenInGame` Bullet true)
      (`Actor.K2_SetActorTransform` Bullet (`self.Spawn Transform`) true false)
      (return))))

(fn `EnableBullet`
  (params (Bullet :type "/Game/Blueprints/Bullets/BP_Bullet Object Reference") (Transform :type "Transform Structure"))
  (`/Engine/EditorBlueprintResources/StandardMacros.IsValid` Bullet
    (:`Is Valid`
      (`Actor.SetActorEnableCollision` Bullet true)
      (`Actor.SetActorHiddenInGame` Bullet false)
      (message `/Game/Interfaces/IBulletEnable.OnBulletEnabled` Bullet Transform)
      (return))))

(fn `GetBullet`
  (returns (Bullet :type "/Game/Blueprints/Bullets/BP_Bullet Object Reference"))
  (locals (CurrentBullet :type "/Game/Blueprints/Bullets/BP_Bullet Object Reference"))
  (bind _output (`|GetArrayItem` (`self.Bullets`)))
  (if (> (`KismetArrayLibrary.Array_Length` (`self.Bullets`)) 0)
    (`/Engine/EditorBlueprintResources/StandardMacros.IsValid` _output
      (:`Is Valid`
        (bind _output_get (set `local.CurrentBullet` _output))
        (`KismetArrayLibrary.Array_RemoveItem` (`self.Bullets`) _output)
        (return _output_get))
      (:`Is Not Valid`
        _)))
  (return null))
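; BP_Bullet is a projectile that flies straight while spinning on its roll axis.
; OnBulletEnabled places it at a given transform, takes that transform's forward vector as Direction and starts both motions.
; Two timelines act as update loops, applying delta-time-scaled roll and swept movement.
; Box overlaps broadcast OnBulletCollide with itself, ignoring actors tagged Bullet or Shooter.
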(event `self.Box.OnComponentBeginOverlap`
  (params (OverlappedComponent :type "PrimitiveComponent Object Reference") (OtherActor :type "Actor Object Reference") (OtherComp :type "PrimitiveComponent Object Reference") (OtherBodyIndex :type Integer) (bFromSweep :type Boolean) (SweepResult :type "HitResult Structure (by ref)"))
  (if (and (not (`self.ActorHasTag` OtherActor "Bullet")) (not (`self.ActorHasTag` OtherActor "Shooter")))
    (`self.OnBulletCollide` self)))

(event `RotateSelf`
  (bind (_returnvalue_roll _returnvalue_pitch _returnvalue_yaw) (`KismetMathLibrary.BreakRotator` (`self.K2_GetActorRotation`)))
  ;[0 0 0] RotateSelf
  (`Timeline|TL_Rotation`
    (:`Update`
      (`self.K2_SetActorRotation` (`KismetMathLibrary.MakeRotator` (+ _returnvalue_roll (* (`GameplayStatics.GetWorldDeltaSeconds`) (`self.RotationSpeed`))) _returnvalue_pitch _returnvalue_yaw)))))

(event `MoveForward`
  ;[0 0 0] MoveForward
  (`Timeline|TL_MoveForward`
    (:`Update`
      (`self.K2_SetActorLocation` (+ (`self.K2_GetActorLocation`) (* (`self.Direction`) (`self.MovementSpeed`) (`GameplayStatics.GetWorldDeltaSeconds`))) true))))

(event `/Game/Interfaces/IBulletEnable.OnBulletEnabled`
  (params (Transform :type "Transform Structure"))
  (`self.K2_SetActorTransform` (`KismetMathLibrary.MakeTransform` Transform_Location Transform_Rotation Transform_Scale))
  (set `self.Direction` (`KismetMathLibrary.Conv_RotatorToVector` Transform_Rotation))
  (`self.RotateSelf`)
  (`self.MoveForward`))

(fn `UserConstructionScript`)
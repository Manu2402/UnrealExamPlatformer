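; BP_Block is a platformer block that the player triggers to release a random object, possibly a powerup or coin.
; A player overlap on Box hides the block and calls GenerateObject, while a hit on Cube disables both components' collision instead of destroying the actor.
; GenerateObject picks from Objects, with an out-of-range roll spawning nothing, corrects height for differing mesh pivots, and has the game mode refresh third-level coins for coin spawns.
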(event `self.ReceiveBeginPlay`
  (bind _asbp_platformer_game_mode (cast `/Game/GameplayFramework/BP_PlatformerGameMode` (`GameplayStatics.GetGameMode`)))
  (set `self.BP_PlatformerGameModeRef` _asbp_platformer_game_mode))

(event `self.Box.OnComponentBeginOverlap`
  (params (OverlappedComponent :type "PrimitiveComponent Object Reference") (OtherActor :type "Actor Object Reference") (OtherComp :type "PrimitiveComponent Object Reference") (OtherBodyIndex :type Integer) (bFromSweep :type Boolean) (SweepResult :type "HitResult Structure (by ref)"))
  ;[0 0 0] Collision
  (if (`self.ActorHasTag` OtherActor "Player")
    (`self.SetActorHiddenInGame` true)
    (`self.GenerateObject`)))

(event `self.Cube.OnComponentHit`
  (params (HitComponent :type "PrimitiveComponent Object Reference") (OtherActor :type "Actor Object Reference") (OtherComp :type "PrimitiveComponent Object Reference") (NormalImpulse :type "Vector Structure") (Hit :type "HitResult Structure (by ref)"))
  ;[0 0 0] I don't destroy the block because may happens some issues about hitting block
  (if (`self.ActorHasTag` OtherActor "Player")
    (`PrimitiveComponent.SetCollisionEnabled` (`self.Box`) "NoCollision")
    (`PrimitiveComponent.SetCollisionEnabled` (`self.Cube`) "NoCollision")))

(event `/Game/Interfaces/IObjectGenerator.GenerateObject`
  (bind _returnvalue (`KismetArrayLibrary.Array_Length` (`self.Objects`)))
  ;[0 0 0] Generate Powerup
  (bind _output_get (set `self.CurrentIndex` (`KismetMathLibrary.RandomIntegerInRange` 0 _returnvalue)))
  (if (< _output_get _returnvalue)
    (bind _output_get_2 (set `self.CurrentObjectType` (`|GetArrayItem` (`self.Objects`) _output_get)))
    (if (!= _output_get_2 "/Game/Blueprints/Collectables/BP_Invincibility.BP_Invincibility_C")
      (set `self.TempOffset` (0.0 0.0 -30.0)))
    (bind _returnvalue_2 (`|SpawnActorFromClass` (`self.CurrentObjectType`) (`KismetMathLibrary.MakeTransform` (+ (`self.K2_GetActorLocation`) (`self.ObjectOffset`) (`self.TempOffset`))) "AdjustIfPossibleButAlwaysSpawn" "MultiplyWithRoot" null null))
    (`/Game/Blueprints/Collectables/BP_CollectableBase.SetPositionAfterSpawn` _returnvalue_2 (`self.ObjectOffset`))
    (if (`self.ActorHasTag` _returnvalue_2 "Coin")
      (`/Game/GameplayFramework/BP_PlatformerGameMode.RefreshAllCoinsThirdLevel` (`self.BP_PlatformerGameModeRef`)))))

(fn `UserConstructionScript`)
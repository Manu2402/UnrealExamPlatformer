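; Boss enemy, extending a parent Blueprint, that gains chase and patrol speed as it loses life.
; A looping timer disables damage-collider overlaps while velocity exceeds the attackable speed, so it is only vulnerable when slow.
; Player overlaps run parent damage logic, scale speeds by lost life and pause capsule overlaps briefly.
; Each hit also flashes the mesh red through a timed FlipFlop material swap.
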(event `self.ReceiveBeginPlay`
  ;[0 0 0] Toggle collisions when is hitted
  (set `self.Life` (`self.BossStartLife`))
  (`parent.ReceiveBeginPlay`)
  (set `self.InitialChaseSpeed` (`self.ChaseSpeed`))
  (set `self.InitialPatrolSpeed` (`self.PatrolSpeed`))
  (`KismetSystemLibrary.K2_SetTimerDelegate` (delegate `ToggleCollision`) (`self.InvincibilityCheckTime`) true))

(event `ToggleCollision`
  ;[0 0 0] Toggle collisions when is hitted
  (bind _output_get (set `self.bIsInvincible?` (> (`KismetMathLibrary.VSize` (`MovementComponent.Velocity` (`self.CharacterMovement`))) (`self.AttackableSpeed`))))
  (set `PrimitiveComponent.bGenerateOverlapEvents` (not _output_get) (`self.DamageCollider`)))

(event `UpdateSpeed`
  (params (NewSpeed :type "Float (double-precision)"))
  (set `CharacterMovementComponent.MaxWalkSpeed` NewSpeed (`self.CharacterMovement`)))

(event `self.DamageCollider.OnComponentBeginOverlap`
  (params (OverlappedComponent :type "PrimitiveComponent Object Reference") (OtherActor :type "Actor Object Reference") (OtherComp :type "PrimitiveComponent Object Reference") (OtherBodyIndex :type Integer) (bFromSweep :type Boolean) (SweepResult :type "HitResult Structure (by ref)"))
  ;[0 0 0] Speed changing when the boss take damage
  (`parent.BodyDamageCollision` OtherActor)
  (if (`self.ActorHasTag` OtherActor "Player")
    (set `self.CurrentDifferenceLife` (- (`self.BossStartLife`) (`self.Life`)))
    (`self.UpdateChaseSpeed`)
    (`self.UpdatePatrolSpeed`)
    (bind _capsulecomponent (`self.CapsuleComponent`)
      (:`then`
        (set `PrimitiveComponent.bGenerateOverlapEvents` false _capsulecomponent)
        (`KismetSystemLibrary.K2_SetTimerDelegate` (delegate `DisableCapsuleCollider`) 1.0)
        (`self.SetMaterialOnTickTime` "/Game/Materials/M_Red.M_Red" (`self.DamageEffectTime`)))
      (:`else`))))

(event `DisableCapsuleCollider`
  ;[0 0 0] Speed changing when the boss take damage
  (set `PrimitiveComponent.bGenerateOverlapEvents` true (`self.CapsuleComponent`)))

(event `UpdateChaseSpeed`
  (set `self.ChaseSpeed` (+ (`self.InitialChaseSpeed`) (* (`self.AdditiveChaseSpeed`) (`self.CurrentDifferenceLife`)))))

(event `UpdatePatrolSpeed`
  (set `self.PatrolSpeed` (+ (`self.InitialPatrolSpeed`) (* (`self.AdditivePatrolSpeed`) (`self.CurrentDifferenceLife`)))))

(event `SetMaterialOnTickTime`
  (params (Material :type "Material Object Reference") (Time :type "Float (double-precision)"))
  (bind _returnvalue (`KismetSystemLibrary.K2_SetTimerDelegate` (delegate `SetMaterialTicked`) (`self.TickTime`) true))
  (`KismetSystemLibrary.K2_SetTimerDelegate` (delegate `StopFlipFlop`) Time))

(event `SetMaterialTicked`
  (bind _mesh (`self.Mesh`))
  (`/Engine/EditorBlueprintResources/StandardMacros.FlipFlop`
    (:`A`
      (`PrimitiveComponent.SetMaterial` _mesh 0 (stale `SetMaterialOnTickTime` Material)))
    (:`B`
      (`PrimitiveComponent.SetMaterial` _mesh 0 null))))

(event `StopFlipFlop`
  (`PrimitiveComponent.SetMaterial` (`self.Mesh`) 0 null)
  (`KismetSystemLibrary.K2_ClearAndInvalidateTimerHandle` (stale `SetMaterialOnTickTime` _returnvalue)))

(fn `UserConstructionScript`
  (`parent.UserConstructionScript`))
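; Base enemy Blueprint that hurts the player on body contact and takes damage through a separate damage collider, launching the player when hit.
; Capsule overlaps toggle Tick, which damages a non-invincible player through BP_PlayerState and grants temporary invincibility.
; At zero life it may spawn a random powerup with pivot-corrected offset, then notifies PlayerState of a boss or regular kill and destroys itself.
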(event `self.ReceiveBeginPlay`
  (bind _asbp_player_state (cast `/Game/GameplayFramework/BP_PlayerState` (`GameplayStatics.GetPlayerState` 0)))
  (set `self.BP_PlayerStateRef` _asbp_player_state))

(event `self.ReceiveTick`
  (params (DeltaSeconds :type "Float (single-precision)"))
  (bind _bp_playerstateref (`self.BP_PlayerStateRef`))
  ;[0 0 0] Tick about damage on the player
  (if (`self.bIsPlayerCollided?`)
    (if (not (`/Game/GameplayFramework/BP_PlayerState.bIsInvincible?` (`self.BP_PlayerStateRef`)))
      (`/Game/GameplayFramework/BP_PlayerState.TakeDamage` _bp_playerstateref 1)
      (`/Game/GameplayFramework/BP_PlayerState.SetInvincibleFor` _bp_playerstateref (`self.InvincibilityTime`)))))

(event `BodyDamageCollision`
  (params (Other :type "Actor Object Reference"))
  (bind _bp_playerstateref (`self.BP_PlayerStateRef`))
  ;[0 0 0] Damage on the enemy
  (if (`self.ActorHasTag` Other "Player")
    (bind _result (`/Engine/EditorBlueprintResources/StandardMacros.DecrementInt` (`self.Life`))
      (:`  `
        (message `/Game/ThirdPersonAssets/ThirdPerson/Blueprints/Interfaces/ILaunch.LaunchCharacterAfterEnemyKilled` Other (`self.JumpForceAfterKill`))
        (if (<= _result 0)
          (`self.SetActorEnableCollision` true)
          (`/Game/Interfaces/IObjectGenerator.GenerateObject`)
          (if (`self.ActorHasTag` "Boss")
            (`/Game/GameplayFramework/BP_PlayerState.BossKilledTrigger` _bp_playerstateref)
            (else
              (`/Game/GameplayFramework/BP_PlayerState.EnemyKilled` _bp_playerstateref)))
          (`self.K2_DestroyActor`))))))

(event `self.DamageCollider.OnComponentBeginOverlap`
  (params (OverlappedComponent :type "PrimitiveComponent Object Reference") (OtherActor :type "Actor Object Reference") (OtherComp :type "PrimitiveComponent Object Reference") (OtherBodyIndex :type Integer) (bFromSweep :type Boolean) (SweepResult :type "HitResult Structure (by ref)"))
  ;[0 0 0] Damage on the enemy
  (`self.BodyDamageCollision` OtherActor))

(event `/Game/Interfaces/IObjectGenerator.GenerateObject`
  (bind _returnvalue (`KismetArrayLibrary.Array_Length` (`self.Objects`)))
  ;[0 0 0] Generate Powerup
  (bind _output_get (set `self.CurrentIndex` (`KismetMathLibrary.RandomIntegerInRange` 0 _returnvalue)))
  (if (< _output_get _returnvalue)
    (bind _output_get_2 (set `self.CurrentObjectType` (`|GetArrayItem` (`self.Objects`) _output_get)))
    (if (!= _output_get_2 "/Game/Blueprints/Collectables/BP_Invincibility.BP_Invincibility_C")
      (set `self.TempOffset` (0.0 0.0 -30.0)))
    (`|SpawnActorFromClass` (`self.CurrentObjectType`) (`KismetMathLibrary.MakeTransform` (+ (`self.K2_GetActorLocation`) (`self.ObjectOffset`) (`self.TempOffset`))) "AdjustIfPossibleButAlwaysSpawn" "MultiplyWithRoot" null null)))

(event `self.CapsuleComponent.OnComponentBeginOverlap`
  (params (OverlappedComponent :type "PrimitiveComponent Object Reference") (OtherActor :type "Actor Object Reference") (OtherComp :type "PrimitiveComponent Object Reference") (OtherBodyIndex :type Integer) (bFromSweep :type Boolean) (SweepResult :type "HitResult Structure (by ref)"))
  (if (`self.ActorHasTag` OtherActor "Player")
    (set `self.bIsPlayerCollided?` true)
    (`self.SetActorTickEnabled` true)))

(event `self.CapsuleComponent.OnComponentEndOverlap`
  (params (OverlappedComponent :type "PrimitiveComponent Object Reference") (OtherActor :type "Actor Object Reference") (OtherComp :type "PrimitiveComponent Object Reference") (OtherBodyIndex :type Integer))
  (if (`self.ActorHasTag` OtherActor "Player")
    (set `self.bIsPlayerCollided?` false)
    (`self.SetActorTickEnabled` false)))

(fn `UserConstructionScript`)
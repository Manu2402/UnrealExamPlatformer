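; AI controller for the Advanced Walker enemy that runs its behavior tree and feeds it player sightings.
; On BeginPlay it stores the controlled walker and starts BT_AdvancedWalker.
; AI Perception updates filter for sight stimuli from Player-tagged actors, setting the blackboard's line-of-sight flag and player reference when seen and clearing both immediately when sight is lost.
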(event `self.ReceiveBeginPlay`
  (bind _asbp_advanced_walker (cast `/Game/Blueprints/Enemies/AdvancedWalker/BP_AdvancedWalker` (`self.K2_GetPawn`)))
  (set `self.OwnerPawn` _asbp_advanced_walker)
  (`self.RunBehaviorTree` "/Game/Blueprints/Enemies/AdvancedWalker/AI/BT_AdvancedWalker.BT_AdvancedWalker"))

(event `self.AIPerception.OnTargetPerceptionUpdated`
  (params (Actor :type "Actor Object Reference") (Stimulus :type "AIStimulus Structure"))
  (bind _blackboard (`self.Blackboard`))
  (bind _blackboard_2 (`self.Blackboard`))
  ;[0 0 0] Sight AI Perception. Handle some variables in blackboard.
  (if (`self.ActorHasTag` Actor "Player")
    (set `self.PerceivedActor` Actor)
    (bind _returnvalue (`AIPerceptionSystem.GetSenseClassForStimulus` Stimulus))
    (if (== _returnvalue "/Script/AIModule.AISense_Sight")
      (if (`.bSuccessfullySensed` (break `AIStimulus` Stimulus))
        (`BlackboardComponent.SetValueAsBool` _blackboard_2 "bHasLineOfSight?" true)
        (`BlackboardComponent.SetValueAsObject` _blackboard_2 "PlayerRef" (`self.PerceivedActor`))
        (else
          (`BlackboardComponent.SetValueAsBool` _blackboard "bHasLineOfSight?" false)
          (`BlackboardComponent.SetValueAsObject` _blackboard "PlayerRef" null))))))

(fn `UserConstructionScript`)
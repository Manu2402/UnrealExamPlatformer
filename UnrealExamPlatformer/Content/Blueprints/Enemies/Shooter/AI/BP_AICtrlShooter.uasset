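; AI controller for the Shooter enemy that runs BT_Shooter and feeds its Blackboard with player sight and fire-range state.
; Sighting the player through AI Perception stores the target and starts a looping range check, which is not cleared when sight is lost.
; The check allows firing inside the distance band and, when too close, caches a fallback point along the player's facing at the band's midpoint.
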(event `self.ReceiveBeginPlay`
  (bind _asbp_shooter (cast `/Game/Blueprints/Enemies/Shooter/BP_Shooter` (`self.K2_GetPawn`)))
  (set `self.OwnerPawn` _asbp_shooter)
  (`self.RunBehaviorTree` "/Game/Blueprints/Enemies/Shooter/AI/BT_Shooter.BT_Shooter")
  (set `self.AverageDistance` (/ (+ (`self.FireDistance`) (`self.DistanceNearPlayer`)) 2.0)))

(event `self.AIPerception.OnTargetPerceptionUpdated`
  (params (Actor :type "Actor Object Reference") (Stimulus :type "AIStimulus Structure"))
  (bind _blackboard (`self.Blackboard`))
  ;[0 0 0] Sight AI Perception. Handle some variables in blackboard. All cases about this enemy.
  (if (`self.ActorHasTag` Actor "Player")
    (set `self.PerceivedActor` Actor)
    (bind _returnvalue (`AIPerceptionSystem.GetSenseClassForStimulus` Stimulus))
    (if (== _returnvalue "/Script/AIModule.AISense_Sight")
      (if (`.bSuccessfullySensed` (break `AIStimulus` Stimulus))
        (`BlackboardComponent.SetValueAsBool` _blackboard "bHasLineOfSight?" true)
        (`BlackboardComponent.SetValueAsObject` _blackboard "PlayerRef" (`self.PerceivedActor`))
        (bind _returnvalue_2 (`KismetSystemLibrary.K2_SetTimerDelegate` (delegate `CheckFireRange`) (`self.FireEvaluationTime`) true))
        (set `self.FireTimer` _returnvalue_2)
        (else
          (`BlackboardComponent.SetValueAsBool` (`self.Blackboard`) "bHasLineOfSight?" false)
          (`BlackboardComponent.SetValueAsBool` (`self.Blackboard`) "bBeyondFireDistance?" false))))))

(event `CheckFireRange`
  (bind _returnvalue (`KismetMathLibrary.Vector_Distance` (`self.K2_GetActorLocation` (`self.PerceivedActor`)) (`self.K2_GetActorLocation` (`self.OwnerPawn`))))
  ;[0 0 0] Sight AI Perception. Handle some variables in blackboard. All cases about this enemy.
  (if (<= _returnvalue (`self.FireDistance`))
    (if (>= _returnvalue (`self.DistanceNearPlayer`))
      (`BlackboardComponent.SetValueAsBool` (`self.Blackboard`) "bHasLineOfSightFire?" true)
      (`self.OnLineOfSightFireChange` true)
      (`BlackboardComponent.SetValueAsBool` (`self.Blackboard`) "bBeyondFireDistance?" true)
      (set `self.bLocationHasCalculated?` false)
      (elif (not (`self.bLocationHasCalculated?`))
        (bind _newlocation (`self.GenerateLocationToTurnBackIntoFireDistance`))
        (set `self.bLocationHasCalculated?` true)
        (`BlackboardComponent.SetValueAsVector` (`self.Blackboard`) "TurnBackToFireDistanceLocation" _newlocation)
        (`BlackboardComponent.SetValueAsBool` (`self.Blackboard`) "bBeyondFireDistance?" true)
        (`BlackboardComponent.SetValueAsBool` (`self.Blackboard`) "bHasLineOfSightFire?" false :!label _label)
        (`self.OnLineOfSightFireChange` false)))
    (else
      (`BlackboardComponent.SetValueAsBool` (`self.Blackboard`) "bBeyondFireDistance?" false)
      (set `self.bLocationHasCalculated?` false)
      (goto _label))))

(fn `GenerateLocationToTurnBackIntoFireDistance`
  (returns (NewLocation :type "Vector Structure"))
  (bind (_returnvalue_roll _returnvalue_pitch _returnvalue_yaw) (`KismetMathLibrary.BreakRotator` (`self.K2_GetActorRotation` (`self.PerceivedActor`))))
  ;[0 0 0] Function that return a new adapted location if the NPC is too near from the player
  (return (+ (* (`self.AverageDistance`) (`KismetMathLibrary.RotateAngleAxis` (1.0 0.0 0.0) _returnvalue_yaw (0.0 0.0 1.0))) (`self.K2_GetActorLocation` (`self.PerceivedActor`)))))

(fn `UserConstructionScript`)
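; Shooter enemy that fires pooled bullets at the player when its line of fire becomes clear.
; Binds to its AI controller's line-of-sight event, relays changes to the Animation Blueprint and shoots once per positive notification.
; Bullets spawn from the mesh's BulletSocket, aimed along the actor-to-player direction, and return to the pool component on collision.
; An UpdateSpeed event sets max walk speed.
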(event `self.ReceiveBeginPlay`
  (`parent.ReceiveBeginPlay`)
  (bind _asbp_aictrl_shooter (cast `/Game/Blueprints/Enemies/Shooter/AI/BP_AICtrlShooter` (`AIBlueprintHelperLibrary.GetAIController` self)))
  (add `/Game/Blueprints/Enemies/Shooter/AI/BP_AICtrlShooter.OnLineOfSightFireChange` _asbp_aictrl_shooter (delegate `LineOfSightFireChanged`))
  (bind _asbp_third_person_character (cast `/Game/ThirdPersonAssets/ThirdPerson/Blueprints/BP_ThirdPersonCharacter` (`GameplayStatics.GetPlayerCharacter` 0)))
  (set `self.BP_ThirdPersonCharacterRef` _asbp_third_person_character))

(event `UpdateSpeed`
  (params (NewSpeed :type "Float (double-precision)"))
  (set `CharacterMovementComponent.MaxWalkSpeed` NewSpeed (`self.CharacterMovement`)))

(event `LineOfSightFireChanged`
  (params (`bHasLineOfSightFire?` :type Boolean))
  ;[0 0 0] Links betweek Behavior Tree and ABP
  (`self.OnHasLineOfSightFireChangedForABP` `bHasLineOfSightFire?`)
  (if `bHasLineOfSightFire?`
    (`self.Shoot`)))

(event `Shoot`
  (bind _bpc_bulletpooling (`self.BPC_BulletPooling`))
  (bind _returnvalue (`SceneComponent.GetSocketTransform` (`self.Mesh`) "BulletSocket" "RTS_World"))
  ;[0 0 0] Calculus about fire distance between this and the player, with handling of object pool
  (bind _bullet (`/Game/Blueprints/Bullets/BPC_BulletPooling.GetBullet` _bpc_bulletpooling))
  (`/Engine/EditorBlueprintResources/StandardMacros.IsValid` _bullet
    (:`Is Valid`
      (`/Game/Blueprints/Bullets/BPC_BulletPooling.EnableBullet` _bpc_bulletpooling _bullet (`KismetMathLibrary.MakeTransform` (.location _returnvalue) (`KismetMathLibrary.Conv_VectorToRotator` (`KismetMathLibrary.Normal` (- (`self.K2_GetActorLocation` (`self.BP_ThirdPersonCharacterRef`)) (`self.K2_GetActorLocation`)))) (.scale _returnvalue)))
      (add `/Game/Blueprints/Bullets/BP_Bullet.OnBulletCollide` _bullet (delegate `BulletCollide`)))))

(event `BulletCollide`
  (params (Bullet :type "/Game/Blueprints/Bullets/BP_Bullet Object Reference"))
  (bind _bpc_bulletpooling (`self.BPC_BulletPooling`))
  ;[0 0 0] Calculus about fire distance between this and the player, with handling of object pool
  (`/Game/Blueprints/Bullets/BPC_BulletPooling.DisableBullet` _bpc_bulletpooling Bullet)
  (`/Game/Blueprints/Bullets/BPC_BulletPooling.AddBullet` _bpc_bulletpooling Bullet))

(fn `UserConstructionScript`
  (`parent.UserConstructionScript`))
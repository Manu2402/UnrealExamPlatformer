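; Base collectable actor that animates into place after spawning, spins, and is picked up by the player.
; SetPositionAfterSpawn moves it vertically via a timeline Lerp to a height derived from the passed offset, then calls RotateSelf.
; RotateSelf uses a second timeline as a ticker, adding yaw scaled by delta time and RotationSpeed.
; Box overlap with a "Player"-tagged actor calls PickUp, which here just destroys the actor.
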(event `self.Box.OnComponentBeginOverlap`
  (params (OverlappedComponent :type "PrimitiveComponent Object Reference") (OtherActor :type "Actor Object Reference") (OtherComp :type "PrimitiveComponent Object Reference") (OtherBodyIndex :type Integer) (bFromSweep :type Boolean) (SweepResult :type "HitResult Structure (by ref)"))
  (if (`self.ActorHasTag` OtherActor "Player")
    (`self.PickUp`)))

(event `RotateSelf`
  (bind (_returnvalue_roll _returnvalue_pitch _returnvalue_yaw) (`KismetMathLibrary.BreakRotator` (`self.K2_GetActorRotation`)))
  ;[0 0 0] Rotate on itself
  (`Timeline|TL_Rotation`
    (:`Update`
      (`self.K2_SetActorRotation` (`KismetMathLibrary.MakeRotator` _returnvalue_roll _returnvalue_pitch (+ _returnvalue_yaw (* (`GameplayStatics.GetWorldDeltaSeconds`) (`self.RotationSpeed`))))))))

(event `PickUp`
  (`self.K2_DestroyActor`))

(event `SetPositionAfterSpawn`
  (params (ObjectOffset :type "Vector Structure"))
  (bind (_returnvalue_x _returnvalue_y _returnvalue_z) (`KismetMathLibrary.BreakVector` (`self.K2_GetActorLocation`)))
  ;[0 0 0] Set position after this object was spawn. All is calculated in order to have total offset = 50 from the block
  (bind _output_get (set `self.StartPositionZ` _returnvalue_z))
  (set `self.EndPositionZ` (- _output_get (- ObjectOffset_Z (`self.SubConstOffset`))))
  (bind (_direction _alpha) (`Timeline|TL_SpawnObject`)
    (:`Update`
      (`self.K2_SetActorLocation` (`KismetMathLibrary.MakeVector` _returnvalue_x _returnvalue_y (`KismetMathLibrary.Lerp` (`self.StartPositionZ`) (`self.EndPositionZ`) _alpha))))
    (:`Finished`
      (`self.RotateSelf`))))

(fn `UserConstructionScript`)
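; BP_Invincibility is a collectable that makes the player temporarily invincible when picked up.
; On BeginPlay it caches the player state and third-person character, and starts its self-rotation.
; PickUp tells BP_PlayerState to apply invincibility for InvincibilityTime, runs the parent pickup logic, then sets a white material on the character for the same duration.
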(event `self.ReceiveBeginPlay`
  (bind _asbp_player_state (cast `/Game/GameplayFramework/BP_PlayerState` (`GameplayStatics.GetPlayerState` 0)))
  (set `self.BP_PlayerStateRef` _asbp_player_state)
  (`self.RotateSelf`)
  (bind _asbp_third_person_character (cast `/Game/ThirdPersonAssets/ThirdPerson/Blueprints/BP_ThirdPersonCharacter` (`GameplayStatics.GetPlayerCharacter` 0)))
  (set `self.BP_ThirdPersonCharacterRef` _asbp_third_person_character))

(event `self.PickUp`
  (`/Game/GameplayFramework/BP_PlayerState.SetInvincibleFor` (`self.BP_PlayerStateRef`) (`self.InvincibilityTime`))
  (`parent.PickUp`)
  (`/Game/ThirdPersonAssets/ThirdPerson/Blueprints/BP_ThirdPersonCharacter.SetMaterialOnTickTime` (`self.BP_ThirdPersonCharacterRef`) "/Game/Materials/M_White.M_White" (`self.InvincibilityTime`)))

(fn `UserConstructionScript`
  (`parent.UserConstructionScript`))
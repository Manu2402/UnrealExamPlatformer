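; BP_Energy is a collectable energy pickup built on a parent class.
; On BeginPlay it caches the player state and HUD references and calls RotateSelf.
; PickUp tells BP_PlayerState that energy was collected, pushes the updated EnergyCounter to the HUD through OnModifiedEnergy, then runs the parent pickup logic.
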(event `self.ReceiveBeginPlay`
  (bind _asbp_player_state (cast `/Game/GameplayFramework/BP_PlayerState` (`GameplayStatics.GetPlayerState` 0)))
  (set `self.BP_PlayerStateRef` _asbp_player_state)
  (`self.RotateSelf`)
  (bind _asbp_hud (cast `/Game/GameplayFramework/BP_HUD` (`PlayerController.GetHUD` (`GameplayStatics.GetPlayerController` 0))))
  (set `self.BP_HUDRef` _asbp_hud))

(event `self.PickUp`
  (bind _bp_playerstateref (`self.BP_PlayerStateRef`))
  (`/Game/GameplayFramework/BP_PlayerState.PickedUpEnergy` _bp_playerstateref)
  (`/Game/Widgets/HUD/WBP_HUD.OnModifiedEnergy` (`/Game/GameplayFramework/BP_HUD.HUDRef` (`self.BP_HUDRef`)) (`/Game/GameplayFramework/BP_PlayerState.EnergyCounter` _bp_playerstateref))
  (`parent.PickUp`))

(fn `UserConstructionScript`
  (`parent.UserConstructionScript`))
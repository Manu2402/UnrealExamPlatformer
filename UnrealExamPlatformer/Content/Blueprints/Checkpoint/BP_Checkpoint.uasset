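; BP_Checkpoint is a level checkpoint that records player progress when an actor tagged Player overlaps its box.
; A per-level flag in the game instance makes the save one-time for Level Two, Level Three and Final Level.
; The first trigger stores the checkpoint location, closes the referenced doors and has the player state snapshot coins and kills.
; Each player overlap also plays a timeline that pitches the flag mesh by frame delta and rotation speed.
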(event `self.ReceiveBeginPlay`
  (bind _asbp_game_instance (cast `/Game/GameplayFramework/BP_GameInstance` (`GameplayStatics.GetGameInstance`)))
  (set `self.BP_GameInstanceRef` _asbp_game_instance)
  (bind _asbp_player_state (cast `/Game/GameplayFramework/BP_PlayerState` (`GameplayStatics.GetPlayerState` 0)))
  (set `self.BP_PlayerStateRef` _asbp_player_state))

(event `self.Box.OnComponentBeginOverlap`
  (params (OverlappedComponent :type "PrimitiveComponent Object Reference") (OtherActor :type "Actor Object Reference") (OtherComp :type "PrimitiveComponent Object Reference") (OtherBodyIndex :type Integer) (bFromSweep :type Boolean) (SweepResult :type "HitResult Structure (by ref)"))
  (bind _bp_gameinstanceref (`self.BP_GameInstanceRef`))
  (bind (_relativerotation_roll _relativerotation_pitch _relativerotation_yaw) (`KismetMathLibrary.BreakRotator` (`SceneComponent.RelativeRotation` (`self.SKM_CheckpointFlag`))))
  ;[0 0 0] By game instance i check the state of all checkpoints
  (if (`self.ActorHasTag` OtherActor "Player")
    (`|ExecutionSequence`
      (:`then_0`
        (switch `/Game/Enums/E_LevelCheckpoint` (`self.LevelCheckpoint`)
          (:`NewEnumerator0`
            (if (not (`/Game/GameplayFramework/BP_GameInstance.bLevelTwoCheckpointIsChecked?` (`self.BP_GameInstanceRef`)))
              (set `/Game/GameplayFramework/BP_GameInstance.bLevelTwoCheckpointIsChecked?` true _bp_gameinstanceref)
              (set `/Game/GameplayFramework/BP_GameInstance.Location` (`self.K2_GetActorLocation`) (`self.BP_GameInstanceRef`) :!label _label)
              (`/Game/Blueprints/Doors/BP_Door.CloseDoors` (`self.BP_DoorRef`))
              (`/Game/GameplayFramework/BP_PlayerState.SetCoinsCounterAndEnemyKillsFromLastCheckpoint` (`self.BP_PlayerStateRef`))))
          (:`NewEnumerator1`
            (if (not (`/Game/GameplayFramework/BP_GameInstance.bLevelThreeCheckpointIsChecked?` (`self.BP_GameInstanceRef`)))
              (set `/Game/GameplayFramework/BP_GameInstance.bLevelThreeCheckpointIsChecked?` true _bp_gameinstanceref)
              (goto _label)))
          (:`NewEnumerator2`
            (if (not (`/Game/GameplayFramework/BP_GameInstance.bFinalLevelCheckpointIsChecked?` (`self.BP_GameInstanceRef`)))
              (set `/Game/GameplayFramework/BP_GameInstance.bFinalLevelCheckpointIsChecked?` true _bp_gameinstanceref)
              (goto _label)))))
      (:`then_1`
        ;[0 0 0] Animation when i check the checkpoint
        (`Timeline|Timeline`
          (:`Update`
            (`SceneComponent.K2_SetRelativeRotation` (`self.SKM_CheckpointFlag`) (`KismetMathLibrary.MakeRotator` _relativerotation_roll (+ _relativerotation_pitch (* (`GameplayStatics.GetWorldDeltaSeconds`) (`self.RotationSpeed`))) _relativerotation_yaw) false false)))))))

(fn `UserConstructionScript`)
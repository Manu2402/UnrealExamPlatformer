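; Double door tied to one of the levels (One, Two, Three or Final) that swings open when that level is exceeded.
; On BeginPlay it binds to the game mode's OnLevelExceeded unless the game instance flags that door as closed, then opens on a matching level.
; A timeline lerps both leaves' yaw by RotationAngle.
; CloseDoors sets the level's closed flag in the game instance and reverses the timeline.
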(event `self.ReceiveBeginPlay`
  (bind _asbp_platformer_game_mode (cast `/Game/GameplayFramework/BP_PlatformerGameMode` (`GameplayStatics.GetGameMode`)))
  (set `self.BP_PlatformerGameModeRef` _asbp_platformer_game_mode)
  (bind _asbp_game_instance (cast `/Game/GameplayFramework/BP_GameInstance` (`GameplayStatics.GetGameInstance`)))
  (bind _output_get (set `self.BP_GameInstanceRef` _asbp_game_instance))
  (switch `/Game/Enums/E_LevelDoors` (`self.LevelDoor`)
    (:`NewEnumerator0`
      (if (not (`/Game/GameplayFramework/BP_GameInstance.bLevelOneDoorIsClosed?` _output_get))
        (add `/Game/GameplayFramework/BP_PlatformerGameMode.OnLevelExceeded` (`self.BP_PlatformerGameModeRef`) (delegate `OnOpenDoor`) :!label _label)))
    (:`NewEnumerator1`
      (if (not (`/Game/GameplayFramework/BP_GameInstance.bLevelTwoDoorIsClosed?` _output_get))
        (goto _label)))
    (:`NewEnumerator2`
      (if (not (`/Game/GameplayFramework/BP_GameInstance.bLevelThreeDoorIsClosed?` _output_get))
        (goto _label)))
    (:`NewEnumerator3`
      (if (not (`/Game/GameplayFramework/BP_GameInstance.bFinalLevelDoorIsClosed?` _output_get))
        (goto _label)))))

(event `OnOpenDoor`
  (params (LevelDoorToOpen :type "/Game/Enums/E_LevelDoors Enum" :default "NewEnumerator0"))
  ;[0 0 0] Select which doors must opens
  (if (`|EnumEquality` LevelDoorToOpen (`self.LevelDoor`))
    (`self.OpenDoors`)))

(event `CloseDoors`
  (bind _bp_gameinstanceref (`self.BP_GameInstanceRef`))
  (bind (_relativerotation_roll _relativerotation_pitch _relativerotation_yaw) (`KismetMathLibrary.BreakRotator` (`SceneComponent.RelativeRotation` (`self.Left`))))
  (bind (_relativerotation_roll_2 _relativerotation_pitch_2 _relativerotation_yaw_2) (`KismetMathLibrary.BreakRotator` (`SceneComponent.RelativeRotation` (`self.Right`))))
  ;[0 0 0] CloseDoors on right doors, always using game instance
  (switch `/Game/Enums/E_LevelDoors` (`self.LevelDoor`)
    (:`NewEnumerator0`
      (set `/Game/GameplayFramework/BP_GameInstance.bLevelOneDoorIsClosed?` true _bp_gameinstanceref)
      ;[0 0 0] OpenDoors Lerping
      (bind (_direction _alpha) (`Timeline|TL_OpenDoors` :!via `Reverse` :!label _label_2)
        (:`Update`
          (`SceneComponent.K2_SetRelativeRotation` (`self.Right`) (`KismetMathLibrary.MakeRotator` _relativerotation_roll _relativerotation_pitch (`KismetMathLibrary.Lerp` (`self.LeftDoorStart`) (`self.LeftDoorEnd`) _alpha)) false false)
          (`SceneComponent.K2_SetRelativeRotation` (`self.Left`) (`KismetMathLibrary.MakeRotator` _relativerotation_roll_2 _relativerotation_pitch_2 (`KismetMathLibrary.Lerp` (`self.RightDoorStart`) (`self.RightDoorEnd`) _alpha)) false false))))
    (:`NewEnumerator1`
      (set `/Game/GameplayFramework/BP_GameInstance.bLevelTwoDoorIsClosed?` true _bp_gameinstanceref)
      (goto _label_2 :!via `Reverse`))
    (:`NewEnumerator2`
      (set `/Game/GameplayFramework/BP_GameInstance.bLevelThreeDoorIsClosed?` true _bp_gameinstanceref)
      (goto _label_2 :!via `Reverse`))
    (:`NewEnumerator3`
      (set `/Game/GameplayFramework/BP_GameInstance.bFinalLevelDoorIsClosed?` true _bp_gameinstanceref)
      (goto _label_2 :!via `Reverse`))))

(event `OpenDoors`
  (bind _rotationangle (`self.RotationAngle`))
  (bind (_relativerotation_roll _relativerotation_pitch _relativerotation_yaw) (`KismetMathLibrary.BreakRotator` (`SceneComponent.RelativeRotation` (`self.Left`))))
  (bind (_relativerotation_roll_2 _relativerotation_pitch_2 _relativerotation_yaw_2) (`KismetMathLibrary.BreakRotator` (`SceneComponent.RelativeRotation` (`self.Right`))))
  ;[0 0 0] OpenDoors Lerping
  (set `self.LeftDoorStart` _relativerotation_yaw)
  (set `self.RightDoorStart` _relativerotation_yaw_2)
  (set `self.LeftDoorEnd` (+ _relativerotation_yaw _rotationangle))
  (set `self.RightDoorEnd` (+ _relativerotation_yaw_2 _rotationangle))
  (goto _label_2))

(fn `UserConstructionScript`)
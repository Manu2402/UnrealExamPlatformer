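; Configurable platform for level design that moves horizontally, moves vertically, rotates or stays idle according to MovementDirection.
; On BeginPlay, timelines lerp location between the start and a Distance offset for ping-pong motion, or add yaw at RotationSpeed scaled by delta time.
; Horizontal motion changes only world X, scaled by the forward vector's X, while vertical changes only Z, scaled by the up vector's Z.
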(event `self.ReceiveBeginPlay`
  (bind (_returnvalue_x _returnvalue_y _returnvalue_z) (`KismetMathLibrary.BreakVector` (`self.K2_GetActorLocation`)))
  (bind _returnvalue_x_2 (`KismetMathLibrary.BreakVector` (`self.K2_GetActorLocation`)))
  (bind (_returnvalue_x_3 _returnvalue_y_2 _returnvalue_z_2) (`KismetMathLibrary.BreakVector` (`self.K2_GetActorLocation`)))
  (bind (_returnvalue_roll _returnvalue_pitch _returnvalue_yaw) (`KismetMathLibrary.BreakRotator` (`self.K2_GetActorRotation`)))
  (bind _returnvalue_x_4 (`KismetMathLibrary.BreakVector` (`KismetMathLibrary.GetForwardVector` (`self.K2_GetActorRotation`))))
  (bind (_returnvalue_x_5 _returnvalue_y_3 _returnvalue_z_3) (`KismetMathLibrary.BreakVector` (`KismetMathLibrary.GetUpVector` (`self.K2_GetActorRotation`))))
  ;[0 0 0] According to the type of movement of the platform it will move in ping pong effect if its type of movement is horizontal/vertical. Instead, if its type of motion is a rotation it will rotate on the Yaw axis at a speed equal to RotationSpeed. In idle the platform rest blocked. All this just to better manage the configuration of platforms during level design.
  (switch `/Game/Enums/E_Movements` (`self.MovementDirection`)
    (:`NewEnumerator0`
      (set `self.StartPosition` _returnvalue_x_2)
      (set `self.EndPosition` (+ _returnvalue_x_2 (* _returnvalue_x_4 (`self.Distance`))))
      (bind (_direction _alpha) (`Timeline|TL_HorizontalMovement`)
        (:`Update`
          (`self.K2_SetActorLocation` (`KismetMathLibrary.MakeVector` (`KismetMathLibrary.Lerp` (`self.StartPosition`) (`self.EndPosition`) _alpha) _returnvalue_y_2 _returnvalue_z_2)))))
    (:`NewEnumerator1`
      (set `self.StartPosition` _returnvalue_z)
      (set `self.EndPosition` (+ _returnvalue_z (* (`self.Distance`) _returnvalue_z_3)))
      (bind (_direction_2 _alpha_2) (`Timeline|TL_VerticalMovement`)
        (:`Update`
          (`self.K2_SetActorLocation` (`KismetMathLibrary.MakeVector` _returnvalue_x_3 _returnvalue_y_2 (`KismetMathLibrary.Lerp` (`self.StartPosition`) (`self.EndPosition`) _alpha_2))))))
    (:`NewEnumerator2`
      (`Timeline|TL_RotationMovement`
        (:`Update`
          (`self.K2_SetActorRotation` (`KismetMathLibrary.MakeRotator` _returnvalue_roll _returnvalue_pitch (+ _returnvalue_yaw (* (`GameplayStatics.GetWorldDeltaSeconds`) (`self.RotationSpeed`))))))))))

(fn `UserConstructionScript`)
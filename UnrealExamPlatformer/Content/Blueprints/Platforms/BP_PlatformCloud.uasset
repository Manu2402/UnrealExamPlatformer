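; Cloud platform, a child of a moving-platform Blueprint, that the player can pass through from below.
; On BeginPlay it forces vertical movement and replaces a near-zero or negative Distance with the default before running the parent logic.
; The Under trigger switches the mesh to overlap-all while a Player-tagged actor is inside and back to block-all on exit, so jumps must fully clear the trigger.
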(event `self.ReceiveBeginPlay`
  ;[0 0 0] Platforms cloud must to have "Movement Direction" as Vertical and must have even a Distance. If Distance has a bad value will be set with a default distance. All this just to better manage the configuration of platforms during level design
  (set `self.MovementDirection` "NewEnumerator1")
  (if (not (>= (`self.Distance`) 0.01))
    (set `self.Distance` (`self.DefaultDistance`)))
  (`parent.ReceiveBeginPlay`))

(event `self.Under.OnComponentBeginOverlap`
  (params (OverlappedComponent :type "PrimitiveComponent Object Reference") (OtherActor :type "Actor Object Reference") (OtherComp :type "PrimitiveComponent Object Reference") (OtherBodyIndex :type Integer) (bFromSweep :type Boolean) (SweepResult :type "HitResult Structure (by ref)"))
  ;[0 0 0] The jump must be accurate because the capsule collider does not conform to the animation of the character, and therefore if the jump does not possess as much offset from the base of the platform the "end overlap" is not called. This could be perfected if the capsule collider were editable or by using the mesh shapes as collision triangles but would be particularly inefficient.
  (`/Engine/EditorBlueprintResources/StandardMacros.IsValid` OtherActor
    (:`Is Valid`
      (if (`self.ActorHasTag` OtherActor "Player")
        (`PrimitiveComponent.SetCollisionProfileName` (`self.StaticMesh`) "OverlapAllDynamic" true)))))

(event `self.Under.OnComponentEndOverlap`
  (params (OverlappedComponent :type "PrimitiveComponent Object Reference") (OtherActor :type "Actor Object Reference") (OtherComp :type "PrimitiveComponent Object Reference") (OtherBodyIndex :type Integer))
  ;[0 0 0] The jump must be accurate because the capsule collider does not conform to the animation of the character, and therefore if the jump does not possess as much offset from the base of the platform the "end overlap" is not called. This could be perfected if the capsule collider were editable or by using the mesh shapes as collision triangles but would be particularly inefficient.
  (`/Engine/EditorBlueprintResources/StandardMacros.IsValid` OtherActor
    (:`Is Valid`
      (if (`self.ActorHasTag` OtherActor "Player")
        (`PrimitiveComponent.SetCollisionProfileName` (`self.StaticMesh`) "BlockAll" true)))))

(fn `UserConstructionScript`
  (`parent.UserConstructionScript`))
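; Player state for a platformer that tracks energy, coins, enemy kills and temporary invincibility.
; Coin and kill totals load from the game instance, and checkpoint snapshots of them are passed to the game mode's death check when damage is taken.
; Pickups, kills and boss defeat notify the game mode, while damage also updates the HUD and flashes the character red.
; Invincibility is a flag cleared by a timer.
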(event `self.ReceiveBeginPlay`
  (set `self.EnergyCounter` (`self.StartEnergy`))
  (bind _asbp_platformer_game_mode (cast `/Game/GameplayFramework/BP_PlatformerGameMode` (`GameplayStatics.GetGameMode`)))
  (set `self.BP_PlatformerGameModeRef` _asbp_platformer_game_mode)
  (bind _asbp_game_instance (cast `/Game/GameplayFramework/BP_GameInstance` (`GameplayStatics.GetGameInstance`)))
  (bind _output_get (set `self.CoinsCounterFromLastCheckpoint` (`/Game/GameplayFramework/BP_GameInstance.CoinsCounter` _asbp_game_instance)))
  (set `self.CoinsCounter` _output_get)
  (bind _output_get_2 (set `self.EnemyKillsFromLastCheckpoint` (`/Game/GameplayFramework/BP_GameInstance.EnemyCounter` _asbp_game_instance)))
  (set `self.EnemyKills` _output_get_2)
  (bind _asbp_third_person_character (cast `/Game/ThirdPersonAssets/ThirdPerson/Blueprints/BP_ThirdPersonCharacter` (`GameplayStatics.GetPlayerCharacter` 0)))
  (set `self.BP_ThirdPersonCharacterRef` _asbp_third_person_character))

(event `PickedUpCoin`
  ;[0 0 0] Check collected coins for game rules
  (bind _result (`/Engine/EditorBlueprintResources/StandardMacros.IncrementInt` (`self.CoinsCounter`))
    (:`  `
      (`/Game/GameplayFramework/BP_PlatformerGameMode.CheckCollectedCoins` (`self.BP_PlatformerGameModeRef`) _result))))

(event `PickedUpEnergy`
  ;[0 0 0] Set Energy Counter with clamp [0, 3]
  (set `self.EnergyCounter` (`KismetMathLibrary.Clamp` (+ (`self.EnergyCounter`) 1) 0 (`self.StartEnergy`))))

(event `TakeDamage`
  (params (Amount :type Integer))
  ;[0 0 0] TakeDamage
  (bind _output_get (set `self.EnergyCounter` (- (`self.EnergyCounter`) Amount)))
  (`/Game/Widgets/HUD/WBP_HUD.OnModifiedEnergy` (`/Game/GameplayFramework/BP_HUD.HUDRef` (`/Game/GameplayFramework/BP_PlatformerGameMode.BP_HUDRef` (`self.BP_PlatformerGameModeRef`))) _output_get)
  (`/Game/ThirdPersonAssets/ThirdPerson/Blueprints/BP_ThirdPersonCharacter.SetMaterialOnTickTime` (`self.BP_ThirdPersonCharacterRef`) "/Game/Materials/M_Red.M_Red" (`self.DamageEffectTime`))
  (`/Game/GameplayFramework/BP_PlatformerGameMode.CheckDeath` (`self.BP_PlatformerGameModeRef`) _output_get (`self.CoinsCounterFromLastCheckpoint`) (`self.EnemyKillsFromLastCheckpoint`)))

(event `SetInvincibleFor`
  (params (Seconds :type "Float (double-precision)"))
  ;[0 0 0] Setting invincibility
  (set `self.bIsInvincible?` true)
  (bind _returnvalue (`KismetSystemLibrary.K2_SetTimerDelegate` (delegate `RemoveInvincibility`) Seconds true)))

(event `RemoveInvincibility`
  ;[0 0 0] Setting invincibility
  (set `self.bIsInvincible?` false)
  (`KismetSystemLibrary.K2_ClearAndInvalidateTimerHandle` (stale `SetInvincibleFor` _returnvalue)))

(event `EnemyKilled`
  ;[0 0 0] Enemy killed
  (bind _result (`/Engine/EditorBlueprintResources/StandardMacros.IncrementInt` (`self.EnemyKills`))
    (:`  `
      (`/Game/GameplayFramework/BP_PlatformerGameMode.CheckEnemiesKilled` (`self.BP_PlatformerGameModeRef`) _result))))

(event `BossKilledTrigger`
  ;[0 0 0] Boss killed
  (`/Game/GameplayFramework/BP_PlatformerGameMode.BossKilled` (`self.BP_PlatformerGameModeRef`)))

(event `SetCoinsCounterAndEnemyKillsFromLastCheckpoint`
  ;[0 0 0] Set values for checkpoints
  (set `self.CoinsCounterFromLastCheckpoint` (`self.CoinsCounter`))
  (set `self.EnemyKillsFromLastCheckpoint` (`self.EnemyKills`)))

(fn `UserConstructionScript`)
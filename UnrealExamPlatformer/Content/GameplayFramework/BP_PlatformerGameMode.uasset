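; Platformer game mode that sets the rules for level progression and player death.
; Coin and enemy-kill thresholds complete the first two stages, both together complete the third, and a boss kill signals the fourth, each through CallOnLevelExceeded.
; On zero energy it saves both counters to the Game Instance and reloads GameLevel.
; CheckFromLevelBP then restores the saved checkpoint position and refreshes the HUD's coins and starting energy.
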(event `self.ReceiveBeginPlay`
  (set `self.LastCheckpointReachedLocation` (`self.InvalidCheckpointLocation`))
  (bind _asbp_third_person_character (cast `/Game/ThirdPersonAssets/ThirdPerson/Blueprints/BP_ThirdPersonCharacter` (`GameplayStatics.GetPlayerCharacter` 0)))
  (set `self.BP_ThirdPersonCharacterRef` _asbp_third_person_character)
  (bind _asbp_player_state (cast `/Game/GameplayFramework/BP_PlayerState` (`GameplayStatics.GetPlayerState` 0)))
  (set `self.BP_PlayerStateRef` _asbp_player_state)
  (bind _asbp_game_instance (cast `/Game/GameplayFramework/BP_GameInstance` (`GameplayStatics.GetGameInstance`)))
  (set `self.BP_GameInstanceRef` _asbp_game_instance)
  (bind _asbp_hud (cast `/Game/GameplayFramework/BP_HUD` (`PlayerController.GetHUD` (`GameplayStatics.GetPlayerController` 0))))
  (set `self.BP_HUDRef` _asbp_hud))

(event `CheckCollectedCoins`
  (params (CoinsCounter :type Integer))
  ;[0 0 0] Rules about collected coins
  (if (>= CoinsCounter (`self.AllCoinsFirstLevel`))
    (if (not (`self.FirstLevelExceeded`))
      (set `self.FirstLevelExceeded` true)
      (`self.OnLevelExceeded` "NewEnumerator0")
      (elif (>= CoinsCounter (`self.AllCoinsThirdLevel`))
        (if (not (`self.Coins_ThirdLevelExceeded`))
          (set `self.Coins_ThirdLevelExceeded` true)
          (`self.CheckExceededThirdLevel`))))))

(event `CheckFromLevelBP`
  (if (`KismetMathLibrary.NotEqualExactly_VectorVector` (`/Game/GameplayFramework/BP_GameInstance.Location` (`self.BP_GameInstanceRef`)) (`self.InvalidCheckpointLocation`))
    (`self.RestorePlayer` (`/Game/GameplayFramework/BP_GameInstance.CoinsCounter` (`self.BP_GameInstanceRef`)))))

(event `CheckDeath`
  (params (EnergyCounter :type Integer) (CoinsCounter :type Integer) (EnemyKillsCounter :type Integer))
  (bind _bp_gameinstanceref (`self.BP_GameInstanceRef`))
  ;[0 0 0] Rules about death + save values for checkpoints and respawn
  (if (<= EnergyCounter 0)
    (set `/Game/GameplayFramework/BP_GameInstance.CoinsCounter` CoinsCounter _bp_gameinstanceref)
    (set `/Game/GameplayFramework/BP_GameInstance.EnemyCounter` EnemyKillsCounter _bp_gameinstanceref)
    (`GameplayStatics.OpenLevel` "GameLevel")))

(event `CheckEnemiesKilled`
  (params (`Enemy Kills` :type Integer))
  ;[0 0 0] Triggers for number of enemies killed
  (if (>= `Enemy Kills` (`self.AllEnemiesSecondLevel`))
    (if (not (`self.SecondLevelExceeded`))
      (set `self.SecondLevelExceeded` true)
      (`self.OnLevelExceeded` "NewEnumerator1")
      (elif (>= `Enemy Kills` (`self.AllEnemiesThirdLevel`))
        (if (not (`self.Enemies_ThirdLevelExceeded`))
          (set `self.Enemies_ThirdLevelExceeded` true)
          (`self.CheckExceededThirdLevel`))))))

(event `CheckExceededThirdLevel`
  ;[0 0 0] Third level conditions
  (if (and (`self.Coins_ThirdLevelExceeded`) (`self.Enemies_ThirdLevelExceeded`))
    (set `self.ThirdLevelExceeded` true)
    (`self.OnLevelExceeded` "NewEnumerator2")))

(event `RefreshAllCoinsThirdLevel`
  (`/Engine/EditorBlueprintResources/StandardMacros.IncrementInt` (`self.AllCoinsThirdLevel`)))

(event `BossKilled`
  (`self.OnLevelExceeded` "NewEnumerator3"))

(event `RestorePlayer`
  (params (CoinsCounter :type Integer))
  (bind _bp_hudref (`self.BP_HUDRef`))
  ;[0 0 0] Trick to retrieve values after death
  (`/Game/ThirdPersonAssets/ThirdPerson/Blueprints/BP_ThirdPersonCharacter.SetPlayerLocation` (`self.BP_ThirdPersonCharacterRef`) (`/Game/GameplayFramework/BP_GameInstance.Location` (`self.BP_GameInstanceRef`)))
  (bind _hudref (`/Game/GameplayFramework/BP_HUD.HUDRef` _bp_hudref)
    (:`then`
      _)
    (:`else`
      (`/Game/GameplayFramework/BP_HUD.SetHUDRef` _bp_hudref)))
  (`/Game/Widgets/HUD/WBP_HUD.OnCoinPickedUp` _hudref CoinsCounter)
  (`/Game/Widgets/HUD/WBP_HUD.OnModifiedEnergy` _hudref (`/Game/GameplayFramework/BP_PlayerState.StartEnergy` (`self.BP_PlayerStateRef`))))

(fn `UserConstructionScript`)
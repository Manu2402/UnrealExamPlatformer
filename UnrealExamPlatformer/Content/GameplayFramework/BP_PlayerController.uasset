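; Player controller that forwards Enhanced Input look, move and jump actions to the possessed pawn.
; It caches the controlled pawn on BeginPlay and relays each action through message calls on that pawn, including jump start and stop.
; The controller holds no movement logic itself, leaving the pawn to implement the response.
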(event `self.ReceiveBeginPlay`
  ;[0 0 0] PlayerController about Pawn
  (set `self.PlayerPawnActorRef` (`self.K2_GetPawn`)))

(event `EnhancedInput|/Game/ThirdPersonAssets/ThirdPerson/Input/Actions/IA_Look`
  (params (ActionValue :type "Vector2D Structure") (ElapsedSeconds :type "Float (double-precision)") (TriggeredSeconds :type "Float (double-precision)") (InputAction :type "InputAction Object Reference" :default "/Game/ThirdPersonAssets/ThirdPerson/Input/Actions/IA_Look.IA_Look"))
  ;[0 0 0] PlayerController about Pawn
  (:`Triggered`
    (message `/Game/ThirdPersonAssets/ThirdPerson/Blueprints/Interfaces/IController.PlayerLook` (`self.PlayerPawnActorRef`) ActionValue_X ActionValue_Y)))

(event `EnhancedInput|/Game/ThirdPersonAssets/ThirdPerson/Input/Actions/IA_Move`
  (params (ActionValue :type "Vector2D Structure") (ElapsedSeconds :type "Float (double-precision)") (TriggeredSeconds :type "Float (double-precision)") (InputAction :type "InputAction Object Reference" :default "/Game/ThirdPersonAssets/ThirdPerson/Input/Actions/IA_Move.IA_Move"))
  ;[0 0 0] PlayerController about Pawn
  (:`Triggered`
    (message `/Game/ThirdPersonAssets/ThirdPerson/Blueprints/Interfaces/IController.PlayerMove` (`self.PlayerPawnActorRef`) ActionValue_X ActionValue_Y)))

(event `EnhancedInput|/Game/ThirdPersonAssets/ThirdPerson/Input/Actions/IA_Jump`
  (params (ActionValue :type Boolean) (ElapsedSeconds :type "Float (double-precision)") (TriggeredSeconds :type "Float (double-precision)") (InputAction :type "InputAction Object Reference" :default "/Game/ThirdPersonAssets/ThirdPerson/Input/Actions/IA_Jump.IA_Jump"))
  (bind _playerpawnactorref (`self.PlayerPawnActorRef`))
  ;[0 0 0] PlayerController about Pawn
  (:`Started`
    (message `/Game/ThirdPersonAssets/ThirdPerson/Blueprints/Interfaces/IController.PlayerJump` _playerpawnactorref))
  (:`Completed`
    (message `/Game/ThirdPersonAssets/ThirdPerson/Blueprints/Interfaces/IController.PlayerStopJumping` _playerpawnactorref)))

(fn `UserConstructionScript`)